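; Test actor for a hatching shader, showing a slowly rotating Sphere lit according to the level's directional light.
; Construction creates a dynamic instance of MI_HatchTest_Inst and runs UpdateMaterial.
; UpdateMaterial looks up a DirectionalLight, passes its forward vector as the "Light Direction" parameter and assigns the material to both Sphere slots.
; Tick repeats that update and adds a fixed, frame-rate-dependent rotation step.
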(event `self.ReceiveTick`
  (params (DeltaSeconds :type "Float (single-precision)"))
  (`self.Update Material`)
  (`self.K2_SetActorRotation` (`KismetMathLibrary.ComposeRotators` (`self.K2_GetActorRotation`) (struct :`Yaw` 1.0))))

(fn `Update Material`
  (bind _sphere (`self.Sphere`))
  (bind _hatch_material (`self.Hatch Material`))
  (bind _returnvalue (`GameplayStatics.GetActorOfClass` "/Script/Engine.DirectionalLight"))
  (`MaterialInstanceDynamic.SetVectorParameterValue` _hatch_material "Light Direction" (`KismetMathLibrary.Conv_VectorToLinearColor` (`SceneComponent.GetForwardVector` (`Light.LightComponent` _returnvalue))))
  (`PrimitiveComponent.SetMaterial` _sphere 0 _hatch_material)
  (`PrimitiveComponent.SetMaterial` _sphere 1 _hatch_material))

(fn `UserConstructionScript`
  (bind _returnvalue (`KismetMaterialLibrary.CreateDynamicMaterialInstance` "/Game/StylizationHW/MI_HatchTest_Inst.MI_HatchTest_Inst"))
  (set `self.Hatch Material` _returnvalue)
  (`self.Update Material`))