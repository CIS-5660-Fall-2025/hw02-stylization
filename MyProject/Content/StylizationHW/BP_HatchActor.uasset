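; Actor with a stylized hatching material on its static mesh that follows the scene's lights.
; Construction creates a dynamic instance of M_SpecialHatch1, and every Tick refreshes it with the first found directional light's forward vector.
; Other lights feed indexed LightDir/LightCol parameters by array position, directional lights leaving index gaps.
; Those values are written crosswise: color into LightDir, forward vector into LightCol.
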(event `self.ReceiveTick`
  (params (DeltaSeconds :type "Float (single-precision)"))
  (`self.Update Material`))

(fn `Init Material`
  (bind _returnvalue (`KismetMaterialLibrary.CreateDynamicMaterialInstance` "/Game/StylizationHW/M_SpecialHatch1.M_SpecialHatch1"))
  (set `self.Hatch Material` _returnvalue)
  (`self.Update Material`))

(fn `Update Light Info`
  (bind _hatch_material (`self.Hatch Material`))
  (bind _outactors (`GameplayStatics.GetAllActorsOfClass` "/Script/Engine.Light"))
  (for (_array_element _array_index) _outactors
    (cast `DirectionalLight` _array_element
      (:`CastFailed`
        (bind _lightcomponent (`Light.LightComponent` _array_element))
        (`MaterialInstanceDynamic.SetVectorParameterValue` _hatch_material (`KismetStringLibrary.Conv_StringToName` (`KismetStringLibrary.Concat_StrStr` "LightDir" (`KismetStringLibrary.Conv_IntToString` _array_index))) (`LightComponentBase.GetLightColor` _lightcomponent))
        (`MaterialInstanceDynamic.SetVectorParameterValue` _hatch_material (`KismetStringLibrary.Conv_StringToName` (`KismetStringLibrary.Concat_StrStr` "LightCol" (`KismetStringLibrary.Conv_IntToString` _array_index))) (`KismetMathLibrary.Conv_VectorToLinearColor` (`SceneComponent.GetForwardVector` _lightcomponent)))
        (`PrimitiveComponent.SetMaterial` (`self.StaticMesh`) 0 _hatch_material)))))

(fn `Update Material`
  (bind _hatch_material (`self.Hatch Material`))
  (bind _returnvalue (`GameplayStatics.GetActorOfClass` "/Script/Engine.DirectionalLight"))
  (`MaterialInstanceDynamic.SetVectorParameterValue` _hatch_material "Light Direction" (`KismetMathLibrary.Conv_VectorToLinearColor` (`SceneComponent.GetForwardVector` (`Light.LightComponent` _returnvalue))))
  (`PrimitiveComponent.SetMaterial` (`self.StaticMesh`) 0 _hatch_material)
  (`self.Update Light Info`))

(fn `UserConstructionScript`
  (`self.Init Material`))